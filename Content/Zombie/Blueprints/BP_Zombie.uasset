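; BP_Zombie is a zombie character that can leap to a given location and be killed by damage.
; Jumpto launches it along a suggested custom-arc velocity toward a point above the destination, then sets a look-at rotation whose target takes only the destination's Z.
; TakeDamage passes the hit to CharacterStatus, prints the remaining health and destroys the actor at zero or below.
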(event EventBeginPlay)

(event Collision|EventActorBeginOverlap
  (params (OtherActor :type Actor%20Object%20Reference)))

(event EventTick
  (params (DeltaSeconds :type Float%20%28single-precision%29)))

(event EventTakeDamage
  (params (HitDamage :type Float%20%28single-precision%29))
  (bind _characterstatus (Variables|Default|GetCharacterStatus))
  (bind _returnvalue (Class|CharacterStatusComponent|GetHealth _characterstatus))
  (Class|CharacterStatusComponent|TakeDamage _characterstatus HitDamage)
  (Development|PrintString (Utilities|String|ToString(Float) _returnvalue))
  (if (<= _returnvalue 0.0)
    (Utilities|IsValid self
      (:Is%20Valid
        (Actor|DestroyActor)))))

(event EventJumpto
  (params (Destination :type Vector :default "0, 0, 0"))
  (bind (_x _y _z) (Math|Vector|BreakVector Destination))
  (bind _returnvalue (Transformation|GetActorLocation))
  (bind _outlaunchvelocity (Game|SuggestProjectileVelocityCustomArc _returnvalue (Math|Vector|MakeVector _x _y (+ _z 1e+02)) 0.0 0.5))
  (Character|LaunchCharacter _outlaunchvelocity true true)
  (Transformation|SetActorRotation (Math|Rotator|FindLookatRotation _returnvalue (Math|Vector|MakeVector 0.0 0.0 _z))))

(fn ConstructionScript)